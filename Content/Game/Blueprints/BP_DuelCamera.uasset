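; Duel camera actor that keeps two players framed by following the midpoint between them.
; Each tick it takes the distance between FirstPlayer and SecondPlayer, floored at MinDistance, and sits that far back along world -X, raised by 0.3 of it.
; It then aims at the midpoint with a LookAt, applying only pitch and yaw.
; Movement is unsmoothed, and a Y-only distance calculation is left unused.
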(event EventTick
  (params (DeltaSeconds :type Float%20%28single-precision%29))
  (bind _returnvalue (Transformation|GetActorTransform))
  (bind _returnvalue_2 (Math|Float|MakeLiteralFloat 2.0))
  (bind _firstplayer (Variables|Default|GetFirstPlayer))
  (bind _secondplayer (Variables|Default|GetSecondPlayer))
  (bind _mindistance (Variables|Default|GetMinDistance))
  (bind _returnvalue_3 (Math|Vector|GetForwardVector (.rotation _returnvalue)))
  (bind _returnvalue_4 (Math|Vector|GetUpVector (.rotation _returnvalue)))
  (bind _returnvalue_5 (Transformation|GetActorLocation _secondplayer))
  (bind _returnvalue_6 (Transformation|GetActorLocation _firstplayer))
  (bind _returnvalue_7 (+ _returnvalue_6 _returnvalue_5))
  (bind _returnvalue_8 (- _returnvalue_6 _returnvalue_5))
  (bind _returnvalue_9 (Math|Vector|VectorLength _returnvalue_8))
  (bind _returnvalue_10 (/ _returnvalue_7 _returnvalue_2))
  (bind _returnvalue_11 (Class|KismetAnimationLibrary|Lookat (Math|Transform|MakeTransform (.location _returnvalue) (.rotation _returnvalue) (.scale _returnvalue)) _returnvalue_10 _returnvalue_3 false _returnvalue_4 0.0))
  (bind (_x _y _z) (Math|Vector|BreakVector _returnvalue_10))
  (bind _returnvalue_12 (Math|Float|Max(Float) _returnvalue_9 _mindistance))
  (Transformation|SetActorLocationAndRotation (Math|Vector|MakeVector (+ _x (* _returnvalue_12 -1.0)) _y (+ (* _returnvalue_12 0.3) _z)) "0, 0, 0")
  (Transformation|SetActorRotation (Math|Rotator|MakeRotator 0.0 (.pitch (.rotation _returnvalue_11)) (.yaw (.rotation _returnvalue_11)))))

(fn ConstructionScript)