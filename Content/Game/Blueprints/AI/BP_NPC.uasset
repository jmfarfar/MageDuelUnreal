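; BP_NPC is an enemy fighter that casts spells and shows its health on the HUD's second-player bar.
; Attack freezes movement, plays a random montage chosen by player distance, then spawns a forward-launched BP_Spell, or plays a defeat montage if dead.
; Mesh hits and TakeDamage both reduce health, but only TakeDamage triggers IsDead, which ragdolls, unpossesses and later destroys the actor.
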(event OnComponentHit(Mesh)
  (params (HitComponent :type Primitive%20Component%20Object%20Reference) (OtherActor :type Actor%20Object%20Reference) (OtherComp :type Primitive%20Component%20Object%20Reference) (NormalImpulse :type Vector :default "0, 0, 0") (Hit :type Hit%20Result%20Structure%20%28by%20ref%29))
  (bind _output_get (Variables|Default|SetHealth (- (Variables|Default|GetHealth) 1e+01)))
  (Default|SetHealthBarInfo (Variables|Default|GetHud) _output_get (Variables|Default|GetMaxHealth) true)
  (if (<= (Variables|Default|GetHealth) 0.0)
    (Variables|Default|SetDead true)))

(event EventAttack
  (bind _returnvalue (Transformation|GetActorTransform))
  (bind _returnvalue_2 (Math|Random|RandomIntegerinRange 0 1))
  (bind _capsulecomponent (Variables|Collision|GetCapsuleComponent))
  (bind _returnvalue_3 (Math|Vector|GetForwardVector _capsulecomponent))
  (bind _returnvalue_4 (== _returnvalue_2 0))
  (if (Variables|Default|GetDead)
    (Animation|Montage|PlayMontage (Variables|Character|GetMesh) "/Game/Game/Models/Characters/Ardid/Animation/AM_Ardid_Defeat.AM_Ardid_Defeat")
    (else
      (CallFunction|DisabledMovement)
      ;[0.4233 0.4678 0.521] Obtener distancia entre enemigo y jugador
      (bind _outactors (Actor|GetAllActorsOfClass "/Game/ThirdPerson/Blueprints/BP_ThirdPersonCharacter.BP_ThirdPersonCharacter_C"))
      (Development|PrintString (Utilities|String|ToString(Float) (Variables|Default|GetHealth)))
      (if (>= (Math|Vector|Distance(Vector) (Transformation|GetActorLocation self) (Transformation|GetActorLocation (Utilities|Array|Get(acopy) _outactors))) 1e+03)
        (if _returnvalue_4
          (Animation|PlayAnimMontage "/Game/ThirdPerson/Character/AttackMontage.AttackMontage" 1.0 "None")
          (Utilities|FlowControl|Delay 0.5)
          (else
            (Animation|PlayAnimMontage "/Game/ThirdPerson/Character/Attack4_M.Attack4_M" 1.0 "None")
            (Utilities|FlowControl|Delay 1.3)))
        (elif _returnvalue_4
          (Animation|PlayAnimMontage "/Game/ThirdPerson/Character/Attack3_M.Attack3_M" 1.0 "None")
          (Utilities|FlowControl|Delay 1.4)
          (else
            (Animation|PlayAnimMontage "/Game/ThirdPerson/Character/Attack2_M.Attack2_M" 1.0 "None")
            (Utilities|FlowControl|Delay 1.0))))
      ;[0.08438 0.5149 0.2159] Lanzar Ataque
      (bind _returnvalue_5 (Game|SpawnActorfromClass "/Game/ThirdPerson/Blueprints/BP_Spell.BP_Spell_C" (Math|Transform|MakeTransform (+ (.location _returnvalue) (* _returnvalue_3 1e+02)) (.rotation _returnvalue) (.scale _returnvalue)) "Undefined" "MultiplyWithRoot" 0 5e+03 _returnvalue_3 0))
      (Default|Spell _returnvalue_5)
      (Utilities|FlowControl|Delay 1.0)
      (CallFunction|EnabledMovement))))

(event EventDestroyFighter
  ;[0.2346 0.2874 0.3419] Destruir enemigo
  (Utilities|FlowControl|Delay 5.0)
  (Actor|DestroyActor))

(fn ConstructionScript)

(fn DisabledMovement
  (Components|Activation|Deactivate (Variables|Character|GetCharacterMovement))
  (return))

(fn EnabledMovement
  (Components|Activation|Activate (Variables|Character|GetCharacterMovement) false)
  (return))

(fn IsDead
  (Physics|SetSimulatePhysics (Variables|Character|GetMesh) true)
  (Collision|SetCollisionEnabled (Variables|Character|GetMesh) "PhysicsOnly")
  (Pawn|Components|CharacterMovement|DisableMovement (Variables|Character|GetCharacterMovement))
  (Pawn|UnPossess (Pawn|GetController))
  (Variables|Default|SetDead true)
  (CallFunction|DestroyFighter)
  (return))

(fn TakeDamage
  (params (Damage :type Float%20%28double-precision%29))
  (bind _output_get (Variables|Default|SetHealth (Math|Float|Clamp(Float) (- (Variables|Default|GetHealth) Damage) 0.0 1e+02)))
  (Default|SetHealthBarInfo (Variables|Default|GetHud) _output_get (Variables|Default|GetMaxHealth) true)
  (if (<= _output_get 0.0)
    (CallFunction|IsDead))
  (return))