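; AI_NPC is an AI controller for NPCs that runs the BT_NPC behavior tree when it possesses a pawn.
; Its perception update writes whether the stimulus was sensed into the CanSeePlayer blackboard key, without checking which actor was perceived.
; A disconnected branch for storing or clearing a TargetActor key remains in the graph but never runs.
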(event OnTargetPerceptionInfoUpdated(AIPerception)
  (params (UpdateInfo :type Actor%20Perception%20Update%20Info%20Structure%20%28by%20ref%29))
  ;[1 1 1] Encontrar al Target y referenciarlo (desactivado)
)

(event OnTargetPerceptionUpdated(AIPerception)
  (params (Actor :type Actor%20Object%20Reference) (Stimulus :type AI%20Stimulus%20Structure))
  (AI|Components|Blackboard|SetValueasBool (AI|GetBlackboard 0) (Utilities|Name|MakeLiteralName "CanSeePlayer") (.bSuccessfullySensed (Utilities|Struct|BreakAIStimulus Stimulus))))

(event EventPossess
  (params (PossessedPawn :type Pawn%20Object%20Reference))
  (AI|RunBehaviorTree "/Game/Game/Blueprints/AI/BT_NPC.BT_NPC"))

(fn ConstructionScript)