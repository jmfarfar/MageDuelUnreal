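; BPC_HealthSystem is a component that tracks an owner's hit points against a maximum.
; TakeDamage subtracts an amount from HP, clamps it at zero and returns whether HP has reached zero.
; Cure adds an amount to HP, capped at MaxHP.
; It has no active event logic, so callers drive all changes and handle the zero-HP result themselves.
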(event EventBeginPlay)

(event EventTick
  (params (DeltaSeconds :type Float%20%28single-precision%29)))

(fn TakeDamage
  (params (Amount :type Float%20%28double-precision%29))
  (bind _output_get (Variables|Default|SetHP (Math|Float|Max(Float) (- (Variables|Default|GetHP) Amount) 0.0)))
  (return (== _output_get 0.0)))

(fn Cure
  (params (Amount :type Float%20%28double-precision%29))
  (Variables|Default|SetHP (Math|Float|Min(Float) (+ (Variables|Default|GetHP) Amount) (Variables|Default|GetMaxHP))))